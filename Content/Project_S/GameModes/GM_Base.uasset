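; Base game mode that holds the server's match settings and player roster, mapping Steam names to team, kill and death data.
; It rebuilds the roster from GI_Project_S on BeginPlay and saves changes back as parallel arrays.
; Login and logout adjust player counts, with logout also removing the player; a LoadingLevel flag suppresses both during ServerTravel.
; UpdateServerValuesOnGameStates passes roster, settings and team scores to a supplied game state.
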(event Custom|SaveServerValues
  (bind _asgi_project_s (Utilities|Casting|CastToGI_Project_S (Game|GetGameInstance)))
  (bind (_name _teams _deaths _kills) (CallFunction|PlayerListtoArrays))
  (Variables|/Game/Project_S/GI_Project_S.GI_Project_S_C|SetPlayerNames _asgi_project_s _name)
  (Variables|/Game/Project_S/GI_Project_S.GI_Project_S_C|SetTeams _asgi_project_s _teams)
  (Variables|/Game/Project_S/GI_Project_S.GI_Project_S_C|SetDeaths _asgi_project_s _deaths)
  (Variables|/Game/Project_S/GI_Project_S.GI_Project_S_C|SetKills _asgi_project_s _kills)
  (Variables|/Game/Project_S/GI_Project_S.GI_Project_S_C|SetRoundTime _asgi_project_s (Variables|Default|GetRoundTime))
  (Variables|/Game/Project_S/GI_Project_S.GI_Project_S_C|SetKillsToWin _asgi_project_s (Variables|Default|GetKillsToWin)))

(event Custom|OnAllPlayerReady)

(event Custom|RemovePlayerServer
  (params (SteamName :type String))
  (Utilities|Map|Remove (Variables|Default|GetPlayerList) SteamName)
  (CallFunction|SaveServerValues))

(event Custom|SetKillsToWin
  (params (KillsToWin :type Integer))
  (Variables|Default|SetKillsToWin KillsToWin)
  (CallFunction|SaveServerValues))

(event Custom|UpdateServerValuesOnGameStates
  (params (GS_Base :type GS%20Base%20Object%20Reference))
  (bind (_playernames _data) (CallFunction|PlayerMapto2Arrays))
  (Default|SetServerValues GS_Base _playernames _data (Variables|Default|GetCurrentPlayerCount) (Variables|Default|GetRoundTime) (Variables|Default|GetKillsToWin) (Variables|Default|GetTeamBrainScore) (Variables|Default|GetTeamMuscleScore)))

(event Custom|OpenLevel
  (params (MapName :type String))
  (Variables|Default|SetbLoadingLevel true)
  (Class|AdvancedSessionsLibrary|ServerTravel MapName false false))

(event Custom|SetRountTime
  (params (NewParam :type Integer))
  (Variables|Default|SetRoundTime NewParam)
  (CallFunction|SaveServerValues))

(event Custom|UpdateSession
  (|UpdateSession 0 100 0 false false false true false true))

(event Custom|ChangeTeamForPlayerServer
  (params (SteamName :type String) (newTeam :type EPlayerTeam%20Enum :default "NewEnumerator0"))
  (Variables|/Game/Project_S/Characters/Player/O_PlayerData.O_PlayerData_C|SetTeam (.Value (Utilities|Map|Find (Variables|Default|GetPlayerList) SteamName)) newTeam)
  (CallFunction|SaveServerValues))

(event Custom|GetStatsFromGameInstace
  (bind _asgi_project_s (Utilities|Casting|CastToGI_Project_S (Game|GetGameInstance)))
  (bind _playerlist (CallFunction|ArraystoPlayerList (Variables|/Game/Project_S/GI_Project_S.GI_Project_S_C|GetPlayerNames _asgi_project_s) (Variables|/Game/Project_S/GI_Project_S.GI_Project_S_C|GetTeams _asgi_project_s) (Variables|/Game/Project_S/GI_Project_S.GI_Project_S_C|GetDeaths _asgi_project_s) (Variables|/Game/Project_S/GI_Project_S.GI_Project_S_C|GetKills _asgi_project_s)))
  (Variables|Default|SetPlayerList _playerlist)
  (Variables|Default|SetRoundTime (Variables|/Game/Project_S/GI_Project_S.GI_Project_S_C|GetRoundTime _asgi_project_s))
  (Variables|Default|SetKillsToWin (Variables|/Game/Project_S/GI_Project_S.GI_Project_S_C|GetKillsToWin _asgi_project_s))
  (bind _keys (Utilities|Map|Keys (Variables|Default|GetPlayerList)))
  (for _array_element _keys
    (Utilities|IsValid (.Value (Utilities|Map|Find (Variables|Default|GetPlayerList) "a")))))

(event EventBeginPlay
  (CallFunction|GetStatsfromGameInstace))

(event EventOnLogout
  (params (ExitingController :type Controller%20Object%20Reference))
  (bind _playerlist (Variables|Default|GetPlayerList))
  (bind _returnvalue (Utilities|Map|Length _playerlist))
  (if (not (Variables|Default|GetbLoadingLevel))
    (bind _output_get (Variables|Default|SetCurrentPlayerCount (- (Variables|Default|GetCurrentPlayerCount) 1)))
    (bind _asplayer_controller (Utilities|Casting|CastToPlayerController ExitingController))
    (bind _returnvalue_2 (Class|AdvancedSteamFriendsLibrary|GetSteamPersonaName (Class|AdvancedSessionsLibrary|GetUniqueNetID _asplayer_controller)))
    (CallFunction|RemovePlayerServer _returnvalue_2)
    (CallFunction|SaveServerValues)
    (if (and (>= _output_get _returnvalue) (!= _returnvalue 0))
      (bind _asgi_project_s (Utilities|Casting|CastToGI_Project_S (Game|GetGameInstance)))
      (Variables|/Game/Project_S/GI_Project_S.GI_Project_S_C|SetWantedPlayerCount _asgi_project_s (+ (Variables|/Game/Project_S/GI_Project_S.GI_Project_S_C|GetWantedPlayerCount _asgi_project_s) -1)))))

(event EventPostLogin
  (params (NewPlayer :type Player%20Controller%20Object%20Reference))
  (if (not (Variables|Default|GetbLoadingLevel))
    (bind _output_get (Variables|Default|SetCurrentPlayerCount (+ (Variables|Default|GetCurrentPlayerCount) 1)))
    (if (>= _output_get (Utilities|Map|Length (Variables|Default|GetPlayerList)))
      (bind _asgi_project_s (Utilities|Casting|CastToGI_Project_S (Game|GetGameInstance)))
      (Variables|/Game/Project_S/GI_Project_S.GI_Project_S_C|SetWantedPlayerCount _asgi_project_s (+ (Variables|/Game/Project_S/GI_Project_S.GI_Project_S_C|GetWantedPlayerCount _asgi_project_s) 1)))))

(fn ConstructionScript)

(fn PlayerListtoArrays
  (bind _playerlist (Variables|Default|GetPlayerList))
  (Utilities|Array|Clear (Variables|Default|GetTempTeams))
  (Utilities|Array|Clear (Variables|Default|GetTempKills))
  (Utilities|Array|Clear (Variables|Default|GetTempDeaths))
  (bind _keys (Utilities|Map|Keys _playerlist))
  (for _array_element _keys
    (Utilities|Array|Add (Variables|Default|GetTempTeams) (Variables|/Game/Project_S/Characters/Player/O_PlayerData.O_PlayerData_C|GetTeam (.Value (Utilities|Map|Find _playerlist _array_element))))
    (Utilities|Array|Add (Variables|Default|GetTempKills) (Variables|/Game/Project_S/Characters/Player/O_PlayerData.O_PlayerData_C|GetKills (.Value (Utilities|Map|Find _playerlist _array_element))))
    (Utilities|Array|Add (Variables|Default|GetTempDeaths) (Variables|/Game/Project_S/Characters/Player/O_PlayerData.O_PlayerData_C|GetDeath (.Value (Utilities|Map|Find _playerlist _array_element)))))
  (return _keys (Variables|Default|GetTempTeams) (Variables|Default|GetTempDeaths) (Variables|Default|GetTempKills)))

(fn ArraystoPlayerList
  (params (SteamNames :type Array%20of%20Strings) (Team :type Array%20of%20EPlayerTeam%20Enums :default "NewEnumerator0") (Deaths :type Array%20of%20Integers) (Kills :type Array%20of%20Integers))
  (Utilities|Map|Clear (Variables|Default|GetTempPlayerList))
  (for (_array_element _array_index) SteamNames
    (bind _returnvalue (Game|ConstructObjectfromClass "/Game/Project_S/Characters/Player/O_PlayerData.O_PlayerData_C"))
    (bind _playerdata (Default|Initalize _returnvalue (Utilities|Array|Get(acopy) Team _array_index) (Utilities|Array|Get(acopy) Kills _array_index) (Utilities|Array|Get(acopy) Deaths _array_index)))
    (Utilities|Map|Add (Variables|Default|GetTempPlayerList) _array_element _playerdata))
  (return (Variables|Default|GetTempPlayerList)))

(fn PlayerMapto2Arrays
  (Utilities|Array|Clear (Variables|Default|GetTempPlayerData))
  (bind _keys (Utilities|Map|Keys (Variables|Default|GetPlayerList)))
  (for _array_element _keys
    (Utilities|Array|Add (Variables|Default|GetTempPlayerData) (.Value (Utilities|Map|Find (Variables|Default|GetTempPlayerList) _array_element))))
  (return _keys (Variables|Default|GetTempPlayerData)))