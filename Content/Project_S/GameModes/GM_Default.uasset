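; Default game mode that runs a timed team match between Brain and Muscle, tracking kills and deaths per Steam name.
; A death credits one team based on the victim's team, but the kill-limit check runs before that increment.
; GameOver, triggered by timer or limit, extends tied rounds by one minute.
; Otherwise it reports the winner through GS_Default and reopens the Lobby as listen server after a short delay.
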(event Custom|AddKillToPlayer
  (params (SteamName :type String))
  (bind _playerlist (Variables|Default|GetPlayerList))
  (bind _value (Utilities|Map|Find _playerlist SteamName))
  (Variables|/Game/Project_S/Characters/Player/O_PlayerData.O_PlayerData_C|SetKills _value (+ (Variables|/Game/Project_S/Characters/Player/O_PlayerData.O_PlayerData_C|GetKills _value) 1))
  (CallFunction|SaveServerValues))

(event Custom|AddPointAndDeath
  (params (SteamName :type String))
  (bind _playerlist (Variables|Default|GetPlayerList))
  (bind _value (Utilities|Map|Find _playerlist SteamName))
  (Variables|/Game/Project_S/Characters/Player/O_PlayerData.O_PlayerData_C|SetDeath _value (+ (Variables|/Game/Project_S/Characters/Player/O_PlayerData.O_PlayerData_C|GetDeath _value) 1))
  (CallFunction|SaveServerValues)
  (CallFunction|CheckforWin)
  (if (Utilities|Enum|Equal(Enum) (Variables|/Game/Project_S/Characters/Player/O_PlayerData.O_PlayerData_C|GetTeam _value) "NewEnumerator0")
    (Variables|Default|SetTeamMuscleScore (+ (Variables|Default|GetTeamMuscleScore) 1))
    (else
      (Variables|Default|SetTeamBrainScore (+ (Variables|Default|GetTeamBrainScore) 1)))))

(event Custom|OnGameStart
  (CallFunction|SetRoundTimer (Math|Conversions|ToFloat(Integer) (Variables|Default|GetRoundTime))))

(event Custom|SetRoundTimer
  (params (TimeInMin :type Float%20%28double-precision%29))
  (bind _returnvalue (Utilities|Time|SetTimerbyFunctionName 0 "GameOver" (* TimeInMin 6e+01))))

(event Custom|CheckForWin
  (if (or (>= (Variables|Default|GetTeamBrainScore) (Variables|Default|GetKillsToWin)) (>= (Variables|Default|GetTeamMuscleScore) (Variables|Default|GetKillsToWin)))
    (CallFunction|GameOver)))

(event Custom|GameOver
  (bind _returnvalue (Game|GetGameState))
  (bind _asgs_default (Utilities|Casting|CastToGS_Default _returnvalue))
  (if (== (Variables|Default|GetTeamBrainScore) (Variables|Default|GetTeamMuscleScore))
    (CallFunction|SetRoundTimer 1.0)
    (else
      (CallFunction|StopTimer)
      (bind _returnvalue_2 (Utilities|Time|SetTimerbyEvent (delegate Custom|BackToLobby) 3.0))
      (if (> (Variables|Default|GetTeamBrainScore) (Variables|Default|GetTeamMuscleScore))
        (Default|OnGameOverMul _asgs_default "NewEnumerator0")
        (else
          (Default|OnGameOverMul _asgs_default "NewEnumerator1"))))))

(event Custom|StopTimer
  (Utilities|Time|ClearandInvalidateTimerbyHandle (stale Custom|SetRoundTimer _returnvalue)))

(event Custom|BackToLobby
  (Game|OpenLevel(byObjectReference) "/Game/Project_S/Maps/Lobby.Lobby" true "listen")
  (Utilities|Time|ClearandInvalidateTimerbyHandle (stale Custom|GameOver _returnvalue_2)))

(event EventUpdateSession
  (|UpdateSession 0 100 0 false false false true false false))

(event EventOnAllPlayerReady
  (bind _asgs_default (Utilities|Casting|CastToGS_Default (Game|GetGameState)))
  (Default|OnAllPlayerReady _asgs_default))

(fn ConstructionScript)