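; Lobby game mode that assigns each joining player to the Brain or Muscle team.
; On PostLogin it tallies the PlayerList map by team and picks the smaller side, with ties going to Brain; the tally variables are not reset in this graph.
; AddPlayerServer stores a new O_PlayerData with team and zeroed kills and deaths under the player's Steam name, then calls SaveServerValues.
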(event Custom|AddPlayerServer
  (params (SteamName :type String) (Team :type EPlayerTeam%20Enum :default "NewEnumerator0"))
  (bind _returnvalue (Game|ConstructObjectfromClass "/Game/Project_S/Characters/Player/O_PlayerData.O_PlayerData_C"))
  (bind _playerdata (Default|Initalize _returnvalue Team))
  (Utilities|Map|Add (Variables|Default|GetPlayerList) SteamName _playerdata)
  (CallFunction|SaveServerValues))

(event EventUpdateSession
  (|UpdateSession 0 100 0 false false false true false true))

(event EventPostLogin
  (params (NewPlayer :type Player%20Controller%20Object%20Reference))
  (bind _playerlist (Variables|Default|GetPlayerList))
  (|CallParentFunction NewPlayer)
  (bind _returnvalue (Class|AdvancedSteamFriendsLibrary|GetSteamPersonaName (Class|AdvancedSessionsLibrary|GetUniqueNetID NewPlayer)))
  (bind _keys (Utilities|Map|Keys _playerlist))
  (for _array_element _keys
    (if (Utilities|Enum|Equal(Enum) (Variables|/Game/Project_S/Characters/Player/O_PlayerData.O_PlayerData_C|GetTeam (.Value (Utilities|Map|Find _playerlist _array_element))) "NewEnumerator0")
      (Variables|Default|SetTeamBrainPlayerCount (+ (Variables|Default|GetTeamBrainPlayerCount) 1))
      (else
        (Variables|Default|SetTeamMusclePlayerCount (+ (Variables|Default|GetTeamMusclePlayerCount) 1)))))
  (if (<= (Variables|Default|GetTeamBrainPlayerCount) (Variables|Default|GetTeamMusclePlayerCount))
    (CallFunction|AddPlayerServer _returnvalue "NewEnumerator0")
    (else
      (CallFunction|AddPlayerServer _returnvalue "NewEnumerator1"))))

(fn ConstructionScript)