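; GM_Everything is a Game Mode Blueprint that reports player joins and departures to the GS_Everything game state.
; On PostLogin it casts the game state and passes the new player's name from PlayerState to AddPlayerServer.
; On logout it does the same with RemovePlayerServer, so players are identified by name.
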(event EventPostLogin
  (params (NewPlayer :type Player%20Controller%20Object%20Reference))
  (Default|AddPlayerServer (.AsGS%20Everything (Utilities|Casting|CastToGS_Everything (Game|GetGameState))) (PlayerState|GetPlayerName (Variables|/Script/Engine.Controller|GetPlayerState NewPlayer))))

(event EventOnLogout
  (params (ExitingController :type Controller%20Object%20Reference))
  (Default|RemovePlayerServer (.AsGS%20Everything (Utilities|Casting|CastToGS_Everything (Game|GetGameState))) (PlayerState|GetPlayerName (Variables|/Script/Engine.Controller|GetPlayerState ExitingController))))

(fn ConstructionScript)