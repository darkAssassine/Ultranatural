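; Player controller that manages a player's team, spawning and match requests in a Salt versus Pepper team game.
; It binds to GS_Everything's ready, reset and team-change events, and looks up its team by player name.
; Respawn replaces and possesses a new CH_Player, using random team start points first and normal spawns afterwards.
; It also forwards kills, team changes, cooldown and match settings to the game state, as a wrapper for non-replicated objects.
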(event Custom|Kick
  (Game|OpenLevel(byObjectReference) "/Game/Project_S/Maps/MainMenu.MainMenu")
  (|DestroySession self))

(event Custom|Respawn
  (bind _returnvalue (Pawn|GetControlledPawn))
  (bind _returnvalue_2 (Game|GetGameState))
  (bind _currentteam (Variables|Default|GetCurrentTeam))
  (bind _asgs_everything (Utilities|Casting|CastToGS_Everything _returnvalue_2))
  (bind _startspawnpointsteamsalt (Variables|/Game/Project_S/GameStates/GS_Everything.GS_Everything_C|GetStartSpawnPointsTeamSalt _asgs_everything))
  (bind _startspawnpointsteampepper (Variables|/Game/Project_S/GameStates/GS_Everything.GS_Everything_C|GetStartSpawnPointsTeamPepper _asgs_everything))
  (bind _outitem (Utilities|Array|Random _startspawnpointsteamsalt))
  (bind _outitem_2 (Utilities|Array|Random _startspawnpointsteampepper))
  (Actor|DestroyActor (Variables|/Game/Project_S/Characters/Player/CH_Player.CH_Player_C|GetCurrentWeapon (.AsCH%20Player (Utilities|Casting|CastToCH_Player _returnvalue))))
  (Actor|DestroyActor _returnvalue)
  (if (Variables|Default|GetbFirstRespawn)
    (if (Utilities|Enum|Equal(Enum) _currentteam "NewEnumerator0")
      (bind _returnvalue_3 (Game|SpawnActorfromClass "/Game/Project_S/Characters/Player/CH_Player.CH_Player_C" (Math|Transform|MakeTransform (.location _outitem) (.rotation _outitem) "1.000000,1.000000,1.000000") "AdjustIfPossibleButAlwaysSpawn" "MultiplyWithRoot" 0 0))
      (Transformation|SetActorTransform _returnvalue_3 (Math|Transform|MakeTransform (.location (Transformation|GetActorTransform _returnvalue_3)) (.rotation _outitem) (.scale (Transformation|GetActorTransform _returnvalue_3))) false true)
      (Pawn|Possess _returnvalue_3)
      (Variables|Default|SetCurrentPlayer _returnvalue_3)
      (Utilities|FlowControl|Delay 0.2)
      (Default|OnStartCooldown _returnvalue_3)
      (else
        (bind _returnvalue_4 (Game|SpawnActorfromClass "/Game/Project_S/Characters/Player/CH_Player.CH_Player_C" (Math|Transform|MakeTransform (.location _outitem_2) (.rotation _outitem_2) "1.000000,1.000000,1.000000") "AdjustIfPossibleButAlwaysSpawn" "MultiplyWithRoot" 0 0))
        (Transformation|SetActorTransform _returnvalue_4 (Math|Transform|MakeTransform (.location (Transformation|GetActorTransform _returnvalue_4)) (.rotation _outitem_2) (.scale (Transformation|GetActorTransform _returnvalue_4))) false true)
        (Pawn|Possess _returnvalue_4)
        (Variables|Default|SetCurrentPlayer _returnvalue_4)
        (Utilities|FlowControl|Delay 0.2)
        (Default|OnStartCooldown _returnvalue_4)))
    (Variables|Default|SetbFirstRespawn false)
    (else
      (bind _spawnpoint (Default|GetNormalSpawn _asgs_everything _currentteam))
      (bind _returnvalue_5 (Game|SpawnActorfromClass "/Game/Project_S/Characters/Player/CH_Player.CH_Player_C" (Math|Transform|MakeTransform (.location _spawnpoint) (.rotation _spawnpoint) "1.000000,1.000000,1.000000") "AdjustIfPossibleButAlwaysSpawn" "MultiplyWithRoot" 0 0))
      (Transformation|SetActorTransform _returnvalue_5 (Math|Transform|MakeTransform (.location (Transformation|GetActorTransform _returnvalue_5)) (.rotation _spawnpoint) (.scale (Transformation|GetActorTransform _returnvalue_5))) false true)
      (Pawn|Possess _returnvalue_5)
      (Variables|Default|SetCurrentPlayer _returnvalue_5)
      (Utilities|FlowControl|Delay 0.2)
      (Default|OnStartCooldown _returnvalue_5))))

(event Custom|TeamChangedServer
  (params (SteamName :type String) (newTeam :type EPlayerTeam%20Enum :default "NewEnumerator0"))
  ;[0.15 0.15 0.15 0.5] Wrapper for gs_everything for object that are not replicated, ugly but workd
  (Default|ChangeTeamforPlayerServer (.AsGS%20Everything (Utilities|Casting|CastToGS_Everything (Game|GetGameState))) SteamName newTeam))

(event Custom|OnTeamChangedServer
  (bind _returnvalue (Game|GetGameState))
  (bind _self self)
  (bind _asgs_everything (Utilities|Casting|CastToGS_Everything _returnvalue))
  (bind _playerstate (Variables|GetPlayerState _self))
  (if (and (Utilities|IsValid _asgs_everything) (Utilities|IsValid _playerstate))
    (bind _team (Default|GetTeamfromPlayer _asgs_everything (PlayerState|GetPlayerName _playerstate)))
    (Variables|Default|SetCurrentTeam _team)))

(event Custom|SetTeamServer
  (bind _returnvalue (Game|GetGameState))
  (bind _asgs_everything (Utilities|Casting|CastToGS_Everything _returnvalue))
  (Variables|Default|SetCurrentTeam (Utilities|Array|Get(acopy) (Variables|/Game/Project_S/GameStates/GS_Everything.GS_Everything_C|GetPlayerTeam _asgs_everything) (Utilities|Array|FindItem (Variables|/Game/Project_S/GameStates/GS_Everything.GS_Everything_C|GetPlayerNames _asgs_everything) (PlayerState|GetPlayerName (Variables|GetPlayerState self)))))
  (CallFunction|Respawn))

(event Custom|Reset
  (Variables|Default|SetbFirstRespawn true)
  (Default|RemoveMapping (.AsCH%20Player (Utilities|Casting|CastToCH_Player (Pawn|GetControlledPawn)))))

(event Custom|AllPlayerReady
  (CallFunction|OnTeamChangedServer)
  (if (Ability|HasAuthority)
    (CallFunction|SetTeamServer)))

(event Custom|AddKillServer
  (Default|AddKillServer (.AsGS%20Everything (Utilities|Casting|CastToGS_Everything (Game|GetGameState))) (PlayerState|GetPlayerName (Variables|/Script/Engine.Controller|GetPlayerState self))))

(event Custom|PlayerMadeKill
  (CallFunction|AddKillServer))

(event Custom|OnTeamChanged
  (CallFunction|OnTeamChangedServer))

(event Custom|TeamChanged
  (params (Name :type String) (newTeam :type EPlayerTeam%20Enum :default "NewEnumerator0"))
  ;[0.15 0.15 0.15 0.5] Wrapper for gs_everything for object that are not replicated, ugly but workd
  (CallFunction|TeamChangedServer Name newTeam))

(event Custom|StartCooldown
  ;[0.15 0.15 0.15 0.5] Wrapper for gs_everything for object that are not replicated, ugly but workd
  (Default|StartCooldown (.AsGS%20Everything (Utilities|Casting|CastToGS_Everything (Game|GetGameState)))))

(event Custom|SetKillsToWin
  (params (KillsToWin :type Integer))
  ;[0.15 0.15 0.15 0.5] Wrapper for gs_everything for object that are not replicated, ugly but workd
  (Default|SetKillstoWin (.AsGS%20Everything (Utilities|Casting|CastToGS_Everything (Game|GetGameState))) KillsToWin))

(event Custom|SetRoundTime
  (params (SetRoundTime :type Integer))
  ;[0.15 0.15 0.15 0.5] Wrapper for gs_everything for object that are not replicated, ugly but workd
  (Default|SetRountTime (.AsGS%20Everything (Utilities|Casting|CastToGS_Everything (Game|GetGameState))) SetRoundTime))

(event EventBeginPlay
  (bind _returnvalue (Game|GetGameState))
  (bind _asgs_everything (Utilities|Casting|CastToGS_Everything _returnvalue))
  (EventDispatchers|BindEventtoAllPlayerReady _asgs_everything (EventDispatchers|CreateEvent :!event Custom|AllPlayerReady))
  (EventDispatchers|BindEventtoReset _asgs_everything (EventDispatchers|CreateEvent :!event Custom|Reset))
  (EventDispatchers|BindEventtoPlayerTeamChanged _asgs_everything (EventDispatchers|CreateEvent :!event Custom|OnTeamChanged))
  (Utilities|FlowControl|Delay 0.2)
  (CallFunction|OnTeamChangedServer))

(fn ConstructionScript)