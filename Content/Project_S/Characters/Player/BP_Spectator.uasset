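; BP_Spectator is a temporary spectator that the player controls until switching back to their character.
; On BeginPlay it adds the IMC_Player Enhanced Input mapping context to the controlling player's subsystem.
; The IA_ChangeToSpectator action makes player controller 0 re-possess the CurrentPlayer stored on PC_Player, restores the in-game UI through HUD_Player, then destroys the spectator.
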(event Input|EnhancedActionEvents|EnhancedInputActionIA_ChangeToSpectator
  (params (ActionValue :type Boolean) (ElapsedSeconds :type Float%20%28double-precision%29) (TriggeredSeconds :type Float%20%28double-precision%29) (InputAction :type Input%20Action%20Object%20Reference :default "/Game/Project_S/Characters/Player/Input/Actions/IA_ChangeToSpectator.IA_ChangeToSpectator"))
  (bind _returnvalue (Game|GetPlayerController 0))
  (bind _aspc_player (Utilities|Casting|CastToPC_Player _returnvalue))
  (Pawn|Possess _returnvalue (Variables|/Game/Project_S/Characters/Player/PC_Player.PC_Player_C|GetCurrentPlayer _aspc_player))
  (Default|AddinGameUI (.AsHUD%20Player (Utilities|Casting|CastToHUD_Player (HUD|GetHUD _aspc_player))))
  (Actor|DestroyActor))

(event EventBeginPlay
  (bind _returnvalue (Pawn|GetController))
  (bind _asplayer_controller (Utilities|Casting|CastToPlayerController _returnvalue))
  (bind _returnvalue_2 (PlayerController|LocalPlayerSubsystems|GetEnhancedInputLocalPlayerSubsystem _asplayer_controller))
  (Utilities|IsValid _returnvalue_2
    (:Is%20Valid
      (Input|AddMappingContext _returnvalue_2 "/Game/Project_S/Characters/Player/Input/IMC_Player.IMC_Player" 0 "(bIgnoreAllPressedKeysUntilRelease=True,bForceImmediately=False,bNotifyUserSettings=False)"))))

(fn ConstructionScript)