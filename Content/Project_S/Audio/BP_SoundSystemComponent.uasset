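; Sound component that plays 3D sounds at a location, attached to a component or from an existing audio component, with optional replication.
; Each entry event plays immediately on the caller, then, if replication is requested, relays through its Server and Mul events.
; The Mul events skip playback where LocalPlayer is locally controlled, so the originating player does not hear the sound twice.
; Particle and system spawn nodes are present but never run.
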(event Custom|Play3DSoundAtLocationServer
  (params (LocalPlayer :type Pawn%20Object%20Reference) (Sound :type Sound%20Base%20Object%20Reference) (Location :type Vector) (Rotation :type Rotator) (VolumeMultiplier :type Float%20%28single-precision%29) (PitchMultiplier :type Float%20%28single-precision%29))
  (CallFunction|Play3DSoundatLocationMul LocalPlayer Sound Location Rotation VolumeMultiplier PitchMultiplier))

(event Custom|Spawn3DSoundAttachedMul
  (params (LocalPlayer :type Pawn%20Object%20Reference) (Sound :type Sound%20Base%20Object%20Reference) (AttachToComponent :type Scene%20Component%20Object%20Reference) (AttachPointName :type Name) (Location :type Vector) (Rotation :type Rotator) (LocationType :type EAttachLocation%20Enum :default "KeepRelativeOffset") (bStopWhenAttachedToDestroyed :type Boolean) (VolumeMultiplier :type Float%20%28single-precision%29) (PitchMultiplier :type Float%20%28single-precision%29))
  (if (not (Pawn|IsLocallyControlled LocalPlayer))
    (Audio|SpawnSoundAttached Sound AttachToComponent AttachPointName Location Rotation LocationType bStopWhenAttachedToDestroyed VolumeMultiplier PitchMultiplier 0.0 0 0)))

(event Custom|Spawn3DSoundAttached
  (params (ShouldReplicate :type Boolean) (LocalPlayer :type Pawn%20Object%20Reference) (Sound :type Sound%20Base%20Object%20Reference) (AttachToComponent :type Scene%20Component%20Object%20Reference) (AttachPointName :type Name) (Location :type Vector) (Rotation :type Rotator) (LocationType :type EAttachLocation%20Enum :default "KeepRelativeOffset") (bStopWhenAttachedToDestroyed :type Boolean) (VolumeMultiplier :type Float%20%28single-precision%29) (PitchMultiplier :type Float%20%28single-precision%29))
  (Audio|SpawnSoundAttached Sound AttachToComponent AttachPointName Location Rotation LocationType bStopWhenAttachedToDestroyed VolumeMultiplier PitchMultiplier 0.0 0 0)
  (if ShouldReplicate
    (CallFunction|Spawn3DSoundAttachedServer LocalPlayer Sound AttachToComponent AttachPointName Location Rotation LocationType bStopWhenAttachedToDestroyed VolumeMultiplier PitchMultiplier)))

(event Custom|Spawn3DSoundAttachedServer
  (params (LocalPlayer :type Pawn%20Object%20Reference) (Sound :type Sound%20Base%20Object%20Reference) (AttachToComponent :type Scene%20Component%20Object%20Reference) (AttachPointName :type Name) (Location :type Vector) (Rotation :type Rotator) (LocationType :type EAttachLocation%20Enum :default "KeepRelativeOffset") (bStopWhenAttachedToDestroyed :type Boolean) (VolumeMultiplier :type Float%20%28single-precision%29) (PitchMultiplier :type Float%20%28single-precision%29))
  (CallFunction|Spawn3DSoundAttachedMul LocalPlayer Sound AttachToComponent AttachPointName Location Rotation LocationType bStopWhenAttachedToDestroyed VolumeMultiplier PitchMultiplier))

(event Custom|PlaySoundFromComponentMul
  (params (Audio%20Component :type Audio%20Component%20Object%20Reference) (LocalPlayer :type Pawn%20Object%20Reference))
  (if (not (Pawn|IsLocallyControlled LocalPlayer))
    (Audio|Components|Audio|Play Audio%20Component 0.0)))

(event Custom|PlaySoundFromComponent
  (params (ShouldReplicate :type Boolean) (LocalPlayer :type Pawn%20Object%20Reference) (Audio%20Component :type Audio%20Component%20Object%20Reference))
  (Audio|Components|Audio|Play Audio%20Component 0.0)
  (if ShouldReplicate
    (CallFunction|PlaySoundfromComponentServer Audio%20Component LocalPlayer)))

(event Custom|PlaySoundFromComponentServer
  (params (Audio%20Component :type Audio%20Component%20Object%20Reference) (LocalPlayer :type Pawn%20Object%20Reference))
  (CallFunction|PlaySoundfromComponentMul Audio%20Component LocalPlayer))

(event Custom|Play3DSoundAtLocationMul
  (params (LocalPlayer :type Pawn%20Object%20Reference) (Sound :type Sound%20Base%20Object%20Reference) (Location :type Vector) (Rotation :type Rotator) (VolumeMultiplier :type Float%20%28single-precision%29) (PitchMultiplier :type Float%20%28single-precision%29))
  (if (not (Pawn|IsLocallyControlled LocalPlayer))
    (Audio|PlaySoundatLocation Sound Location Rotation VolumeMultiplier PitchMultiplier 0.0 0 0 0 0)))

(event Custom|Play3DSoundAtLocation
  (params (ShouldReplicate :type Boolean) (LocalPlayer :type Pawn%20Object%20Reference) (Sound :type Sound%20Base%20Object%20Reference) (Location :type Vector) (Rotation :type Rotator) (VolumeMultiplier :type Float%20%28single-precision%29) (PitchMultiplier :type Float%20%28single-precision%29))
  (Audio|PlaySoundatLocation Sound Location Rotation VolumeMultiplier PitchMultiplier 0.0 0 0 0 0)
  (if ShouldReplicate
    (CallFunction|Play3DSoundatLocationServer LocalPlayer Sound Location Rotation VolumeMultiplier PitchMultiplier)))