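; BP_Forward_JumpPad is a jump pad that launches characters in a configurable direction when they overlap its box trigger.
; The construction script rotates an arrow component to DirectionRotation, and the overlap launches the character along that arrow's forward vector scaled by BoostStrength, overriding existing velocity.
; Each launch also plays the pad's audio through the BP sound system component with replication requested.
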(event OnComponentBeginOverlap(Box)
  (params (OverlappedComponent :type Primitive%20Component%20Object%20Reference) (OtherActor :type Actor%20Object%20Reference) (OtherComp :type Primitive%20Component%20Object%20Reference) (OtherBodyIndex :type Integer) (bFromSweep :type Boolean) (SweepResult :type Hit%20Result%20Structure%20%28by%20ref%29))
  (bind _ascharacter (Utilities|Casting|CastToCharacter OtherActor))
  (Character|LaunchCharacter _ascharacter (* (Math|Vector|GetForwardVector (Variables|Default|GetArrow)) (Variables|Default|GetBoostStrength)) true true)
  (Default|PlaySoundfromComponent (Variables|Default|GetBP_SoundSystemComponent) true (Game|Player|GetPlayerPawn 0) (Variables|Default|GetAudio_JumpPad)))

(event EventBeginPlay)

(event Collision|EventActorBeginOverlap
  (params (OtherActor :type Actor%20Object%20Reference)))

(event EventTick
  (params (DeltaSeconds :type Float%20%28single-precision%29)))

(fn ConstructionScript
  (Transformation|SetRelativeRotation (Variables|Default|GetArrow) (Variables|Default|GetDirectionRotation) false false))