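; BP_SpawnPoint is a team spawn point that registers itself with the game state and reports whether a given team can spawn there.
; On BeginPlay, the server passes the actor's transform, Team and self reference to GS_Everything through AddSpawnPoint.
; PossibleSpawnForPlayerFromTeam refuses the spawn if any overlapping CH_Player's controller belongs to another team, and allows it otherwise.
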(event Custom|Set%20Spawn%20Points
  (if (Networking|IsServer)
    (bind _asgs_everything (Utilities|Casting|CastToGS_Everything (Game|GetGameState)))
    (Default|AddSpawnPoint _asgs_everything (Transformation|GetActorTransform) (Variables|Default|GetTeam) self)))

(event EventBeginPlay
  (CallFunction|SetSpawnPoints))

(fn ConstructionScript)

(fn PossibleSpawnforPlayerfromTeam
  (params (TeamToSpawn :type EPlayerTeam%20Enum :default "NewEnumerator0"))
  (for _array_element (Collision|GetOverlappingActors "/Game/Project_S/Characters/Player/CH_Player.CH_Player_C" :!class /Script/Engine.Actor)
    (if (Utilities|Enum|NotEqual(Enum) TeamToSpawn (Variables|/Game/Project_S/Characters/Player/PC_Player.PC_Player_C|GetCurrentTeam (.AsPC%20Player (Utilities|Casting|CastToPC_Player (Pawn|GetController _array_element)))))
      (return false)))
  (return true))