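; BP_Weapon is a hitscan gun, apparently a common base, that manages ammo, timed cooldown and reload.
; TryShoot triggers a camera sphere trace, then cooldown re-arms firing or calls the player's reload when empty.
; HandleHit damages enemy players with headshot crits, sends hit feedback and reports predicted kills to GS_Everything.
; Trails and impacts spawn locally and via Server/Multi events, with multicast trails skipping the locally controlled shooter.
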(event Custom|LowAmmoSFX
  (if (<= (Variables|Default|GetCurrentAmmo) 5)
    (Default|PlaySoundfromComponent (Variables|Default|GetBP_SoundSystemComponent) true (Game|Player|GetPlayerPawn 0) (Variables|Default|GetAudio_empty%20Magazine))))

(event Custom|HandleHit
  (params (Hit :type Hit%20Result%20Structure) (bHit :type Boolean) (Player :type CH%20Player%20Object%20Reference))
  (bind _returnvalue (Pawn|GetController Player))
  (bind (_bblockinghit _binitialoverlap _time _distance _location _impactpoint _normal _impactnormal _physmat _hitactor _hitcomponent) (Collision|BreakHitResult Hit))
  (bind _returnvalue_2 (Transformation|GetActorTransform Player))
  (bind _returnvalue_3 (Game|GetPlayerController 0))
  (bind _critdamage (Variables|Default|GetCritDamage))
  (bind _damage (Variables|Default|GetDamage))
  (bind _playername (Class|AdvancedSessionsLibrary|GetPlayerName _returnvalue_3))
  (bind _playerstate (Variables|/Script/Engine.Controller|GetPlayerState _returnvalue))
  (bind _returnvalue_4 (PlayerState|GetPlayerName _playerstate))
  (if bHit
    (CallFunction|HitEffectsServer Hit)
    (CallFunction|HitEffectLocal Hit)
    (bind _asch_player (Utilities|Casting|CastToCH_Player _hitactor)
      (:then
        (if (Utilities|Enum|NotEqual(Enum) (Variables|/Game/Project_S/Characters/Player/CH_Player.CH_Player_C|GetCurrentTeam _asch_player) (Variables|/Game/Project_S/Characters/Player/CH_Player.CH_Player_C|GetCurrentTeam Player))
          (if (Components|ComponentHasTag _hitcomponent "Head")
            (if (and (Variables|/Game/Project_S/Characters/Player/CH_Player.CH_Player_C|GetbAliveNotRep _asch_player) (Variables|/Game/Project_S/Characters/Player/CH_Player.CH_Player_C|GetbAlive _asch_player))
              (bind _newparam (Default|WouldbeDeadifTakeDamage _asch_player _critdamage))
              (CallFunction|DamagePlayer _asch_player _critdamage _returnvalue_4 (.location _returnvalue_2))
              (if _newparam
                (Variables|/Game/Project_S/Characters/Player/CH_Player.CH_Player_C|SetbAliveNotRep _asch_player false)
                (Default|HandleHitFeedback Player "NewEnumerator3")
                (CallFunction|AddKilltoPlayesr _playername)
                (else
                  (Default|HandleHitFeedback Player "NewEnumerator1" :!label _label)))
              (else
                (goto _label)))
            (elif (Variables|/Game/Project_S/Characters/Player/CH_Player.CH_Player_C|GetbAlive _asch_player)
              (bind _newparam_2 (Default|WouldbeDeadifTakeDamage _asch_player _damage))
              (CallFunction|DamagePlayer _asch_player _damage _returnvalue_4 (.location _returnvalue_2))
              (if _newparam_2
                (Variables|/Game/Project_S/Characters/Player/CH_Player.CH_Player_C|SetbAliveNotRep _asch_player false)
                (Default|HandleHitFeedback Player "NewEnumerator3")
                (CallFunction|AddKilltoPlayesr _playername)
                (else
                  (Default|HandleHitFeedback Player "NewEnumerator2" :!label _label_2)))
              (else
                (goto _label_2))))
          (else
            (Default|HandleHitFeedback Player "NewEnumerator4"))))
      (:CastFailed
        (Default|HandleHitFeedback Player "NewEnumerator0")))
    (else
      (Default|HandleHitFeedback Player "NewEnumerator0"))))

(event Custom|HitEffectLocal
  (params (Hit :type Hit%20Result%20Structure%20%28by%20ref%29))
  (bind (_bblockinghit _binitialoverlap _time _distance _location _impactpoint _normal _impactnormal _physmat _hitactor) (Collision|BreakHitResult Hit))
  (Utilities|Casting|CastToCH_Player _hitactor
    (:then
      (Niagara|SpawnSystematLocation "/Game/Project_S/VFX/BloodSplatter/PS_VFXBloodSplatter.PS_VFXBloodSplatter" _location "0, 0, 0" "1.000000,1.000000,1.000000" false))
    (:CastFailed
      (Effects|SpawnEmitteratLocation "/Game/PlaceHolderAssets/StarterContent/Particles/P_Explosion.P_Explosion" _location "0, 0, 0" (Variables|Default|GetVFXScale)))))

(event Custom|Reload
  (bind _returnvalue (Utilities|Time|SetTimerbyEvent (delegate Custom|OnReloadOver) (Variables|Default|GetReloadTime)))
  (Variables|Default|SetReloadTimerHandle _returnvalue)
  (Utilities|FlowControl|Delay 0.1)
  (Default|PlaySoundfromComponent (Variables|Default|GetBP_SoundSystemComponent) true (Game|Player|GetPlayerPawn 0) (Variables|Default|GetAudio_reloading)))

(event Custom|StopReloadTimer
  (Utilities|Time|ClearandInvalidateTimerbyHandle (stale Custom|Reload _returnvalue)))

(event Custom|OnReloadOver
  (Variables|Default|SetbShoot true)
  (Variables|Default|SetCurrentAmmo (Variables|Default|GetMaxAmmo))
  (CallFunction|StopReloadTimer))

(event Custom|Reset
  (Variables|Default|SetCurrentAmmo (Variables|Default|GetMaxAmmo)))

(event Custom|SpawnWeaponTrailMul
  (params (Direction :type Vector) (Start :type Vector) (NewParam :type CH%20Player%20Object%20Reference))
  (if (not (Pawn|IsLocallyControlled NewParam))
    (bind _returnvalue (Niagara|SpawnSystematLocation "/Game/Project_S/Weapons/Common/NS_BulltetTrace.NS_BulltetTrace" Start))
    (Niagara|SetNiagaraVariable(Vector3) _returnvalue "Direction" Direction)
    (Niagara|SetNiagaraVariable(Vector3) _returnvalue "DirectionMinus" (Math|Vector|NegateVector Direction))))

(event Custom|DamagePlayer
  (params (Player :type CH%20Player%20Object%20Reference) (Damage :type Integer) (AttackerName :type String) (Pos :type Vector))
  (Default|TakeDamage Player Damage AttackerName Pos))

(event Custom|SpawnWeaponTrailLocal
  (params (Start :type Vector) (End :type Vector) (NewParam :type CH%20Player%20Object%20Reference))
  (bind _weaponmesh (Variables|Default|GetWeaponMesh))
  (bind _returnvalue (Transformation|GetSocketLocation _weaponmesh "Ammo"))
  (bind _returnvalue_2 (- End _returnvalue))
  (bind _returnvalue_3 (Math|Vector|Normalize _returnvalue_2))
  (CallFunction|SpawnWeaponTrailServer _returnvalue_3 (+ Start (* _returnvalue_3 "10.000000,10.000000,10.000000")) NewParam)
  (bind _returnvalue_4 (Niagara|SpawnSystematLocation "/Game/Project_S/Weapons/Common/NS_BulltetTrace.NS_BulltetTrace" Start))
  (Niagara|SetNiagaraVariable(Vector3) _returnvalue_4 "Direction" _returnvalue_3)
  (Niagara|SetNiagaraVariable(Vector3) _returnvalue_4 "DirectionMinus" (Math|Vector|NegateVector _returnvalue_3)))

(event Custom|AddKillToPlayesr
  (params (NewParam :type String))
  (Default|AddKillServer (.AsGS%20Everything (Utilities|Casting|CastToGS_Everything (Game|GetGameState))) NewParam))

(event Custom|SpawnWeaponTrailServer
  (params (Direction :type Vector) (Start :type Vector) (NewParam :type CH%20Player%20Object%20Reference))
  (CallFunction|SpawnWeaponTrailMul Direction Start NewParam))

(event Custom|MuzzleFlashServer
  (CallFunction|MuzzleFlashMulti))

(event Custom|Shoot
  (params (CamPos :type Vector) (CamDir :type Vector) (Player :type CH%20Player%20Object%20Reference))
  (bind _weaponmesh (Variables|Default|GetWeaponMesh))
  (bind _returnvalue (Transformation|GetSocketLocation _weaponmesh "Ammo"))
  (Default|SpawnSystemAttached (Variables|Default|GetBP_VFXSpawnComponent) true (Game|Player|GetPlayerPawn 0) "/Game/VFX_Muzzle_Flashes/ParticleSystems/UserVersionsAtSingleLoop/UpdatedVersions/First_Person_Versions/FXS_ShotgunMuzzle_FirstPerson.FXS_ShotgunMuzzle_FirstPerson" (Variables|Default|GetWeaponMesh) "MuzzleFlash" "0, 0, 0" "0, 0, 0" false)
  (bind (_outhit _returnvalue_2) (Collision|SphereTraceForObjects CamPos (+ CamPos (* CamDir (Variables|Default|GetRange))) (Variables|Default|GetRadius) (Utilities|Array|MakeArray "ObjectTypeQuery2" "ObjectTypeQuery1" "ObjectTypeQuery4" "ObjectTypeQuery8") false (Utilities|Array|MakeArray Player) "None"))
  (if _returnvalue_2
    (CallFunction|SpawnWeaponTrailLocal _returnvalue (.Location (Collision|BreakHitResult _outhit)) Player)
    (CallFunction|HandleHit _outhit _returnvalue_2 Player)
    (else
      (CallFunction|SpawnWeaponTrailLocal _returnvalue (.TraceEnd (Collision|BreakHitResult _outhit)) Player)
      (CallFunction|HandleHit _outhit _returnvalue_2 Player)))
  (Default|PlaySoundfromComponent (Variables|Default|GetBP_SoundSystemComponent) true (Game|Player|GetPlayerPawn 0) (Variables|Default|GetShootSound)))

(event Custom|HitEffectsServer
  (params (Hit :type Hit%20Result%20Structure))
  (CallFunction|HitEffectsMul Hit))

(event Custom|MuzzleFlashMulti
  (bind _weaponmesh (Variables|Default|GetWeaponMesh))
  (bind _returnvalue (Transformation|GetSocketTransform _weaponmesh "MuzzleFlash" "RTS_World"))
  (Niagara|SpawnSystemAttached "/Game/VFX_Muzzle_Flashes/ParticleSystems/UserVersionsAtSingleLoop/LEGACY_VERSIONS/First_Person_Versions/FXS_ShotgunMuzzle_FirstPerson.FXS_ShotgunMuzzle_FirstPerson" (Variables|Default|GetDefaultSceneRoot) "Ammo" (+ (.location _returnvalue) (* (Math|Vector|GetForwardVector (.rotation _returnvalue)) "")) (.rotation _returnvalue) "KeepWorldPosition" true))

(event Custom|OnCooldownOver
  (CallFunction|StopTimer)
  (if (> (Variables|Default|GetCurrentAmmo) 0)
    (Variables|Default|SetbShoot true)
    (else
      (Variables|Default|SetbShoot false)
      (Default|Reload (stale Custom|TryShoot Player)))))

(event Custom|HitEffectsMul
  (params (Hit :type Hit%20Result%20Structure%20%28by%20ref%29))
  (bind (_bblockinghit _binitialoverlap _time _distance _location _impactpoint _normal _impactnormal _physmat _hitactor) (Collision|BreakHitResult Hit))
  (if (!= (Game|GetInstigator) self)
    (Utilities|Casting|CastToCH_Player _hitactor
      (:then
        (Niagara|SpawnSystematLocation "/Game/Project_S/VFX/BloodSplatter/PS_VFXBloodSplatter.PS_VFXBloodSplatter" _location "0, 0, 0" "1.000000,1.000000,1.000000" false))
      (:CastFailed
        (Effects|SpawnEmitteratLocation "/Game/PlaceHolderAssets/StarterContent/Particles/P_Explosion.P_Explosion" _location "0, 0, 0" (Variables|Default|GetVFXScale))))))

(event Custom|StopTimer
  (Utilities|Time|ClearandInvalidateTimerbyHandle (stale Custom|TryShoot _returnvalue)))

(event Custom|TryShoot
  (params (CameraPos :type Vector) (CameraDIr :type Vector) (Player :type CH%20Player%20Object%20Reference))
  (if (Variables|Default|GetbShoot)
    (Variables|Default|SetbShoot false)
    (bind _returnvalue (Utilities|Time|SetTimerbyEvent (delegate Custom|OnCooldownOver) (Variables|Default|GetCooldown)))
    (Variables|Default|SetCurrentAmmo (- (Variables|Default|GetCurrentAmmo) 1))
    (CallFunction|StopReloadTimer)
    (CallFunction|Shoot CameraPos CameraDIr Player)
    (CallFunction|LowAmmoSFX)))

(fn ConstructionScript)

(fn GetEndPointfromCameraRaycast
  (params (CamPos :type Vector) (CamDir :type Vector) (PlayerToIgnore :type CH%20Player%20Object%20Reference))
  (bind (_outhits _returnvalue) (Collision|MultiSphereTraceForObjects CamPos (+ CamPos (* CamDir (Variables|Default|GetRange))) (Variables|Default|GetRadius) (Utilities|Array|MakeArray "ObjectTypeQuery2" "ObjectTypeQuery1" "ObjectTypeQuery4" "ObjectTypeQuery8") false (Utilities|Array|MakeArray PlayerToIgnore) "None"))
  (if _returnvalue
    (return (.Location (Collision|BreakHitResult (Utilities|Array|Get(acopy) _outhits (Utilities|Array|LastIndex _outhits)))) _returnvalue (Utilities|Array|Get(acopy) _outhits (Utilities|Array|LastIndex _outhits)))
    (else
      (return (.TraceEnd (Collision|BreakHitResult (Utilities|Array|Get(acopy) _outhits (Utilities|Array|LastIndex _outhits)))) _returnvalue (Utilities|Array|Get(acopy) _outhits (Utilities|Array|LastIndex _outhits))))))