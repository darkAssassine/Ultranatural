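; Component that spawns Niagara systems and particle emitters, at a location or attached to a component, with optional replication to other players.
; Each entry event spawns the effect locally at once, then, if ShouldReplicate is set, passes it through a Server event to a Mul event.
; The Mul events respawn the effect only where the passed pawn is not locally controlled, so the originating player does not see it twice.
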(event Custom|SpawnSystemAttachedMul
  (params (LocalPawn :type Pawn%20Object%20Reference) (NiagaraTemplate :type Niagara%20System%20Object%20Reference) (AttachToComponent :type Scene%20Component%20Object%20Reference) (AttachPointName :type Name) (Location :type Vector) (Rotation :type Rotator) (bAutoDestroy :type Boolean))
  (if (not (Pawn|IsLocallyControlled LocalPawn))
    (Niagara|SpawnSystemAttached NiagaraTemplate AttachToComponent AttachPointName Location Rotation "KeepRelativeOffset" bAutoDestroy)))

(event Custom|SpawnEmitterAtLocation
  (params (ShouldReplicate :type Boolean) (LocalPawn :type Pawn%20Object%20Reference) (EmitterTemplate :type Particle%20System%20Object%20Reference) (Location :type Vector) (Rotation :type Rotator) (Scale :type Vector) (bAutoDestroy :type Boolean))
  (Effects|SpawnEmitteratLocation EmitterTemplate Location Rotation Scale bAutoDestroy)
  (if ShouldReplicate
    (CallFunction|SpawnEmitteratLocationServer LocalPawn EmitterTemplate Location Rotation Scale bAutoDestroy)))

(event Custom|SpawnEmitterAtLocationServer
  (params (PlayerFormClient :type Pawn%20Object%20Reference) (EmitterTemplate :type Particle%20System%20Object%20Reference) (Location :type Vector) (Rotation :type Rotator) (Scale :type Vector) (bAutoDestroy :type Boolean))
  (CallFunction|SpawnEmitteratLocationMul PlayerFormClient EmitterTemplate Location Rotation Scale bAutoDestroy))

(event Custom|SpawnEmitterAtLocationMul
  (params (PlayerFromClient :type Pawn%20Object%20Reference) (EmitterTemplate :type Particle%20System%20Object%20Reference) (Location :type Vector) (Rotation :type Rotator) (Scale :type Vector) (bAutoDestroy :type Boolean))
  (if (not (Pawn|IsLocallyControlled PlayerFromClient))
    (Effects|SpawnEmitteratLocation EmitterTemplate Location Rotation Scale bAutoDestroy)))

(event Custom|SpawnSystemAttached
  (params (ShouldReplicate :type Boolean) (LocalPawn :type Pawn%20Object%20Reference) (NiagaraTemplate :type Niagara%20System%20Object%20Reference) (AttachToComponent :type Scene%20Component%20Object%20Reference) (AttachPointName :type Name) (Location :type Vector) (Rotation :type Rotator) (bAutoDestroy :type Boolean))
  (Niagara|SpawnSystemAttached NiagaraTemplate AttachToComponent AttachPointName Location Rotation "KeepRelativeOffset" bAutoDestroy)
  (if ShouldReplicate
    (CallFunction|SpawnSystemAttachedServer LocalPawn NiagaraTemplate AttachToComponent AttachPointName Location Rotation bAutoDestroy)))

(event Custom|SpawnSystemAttachedServer
  (params (LocalPawn :type Pawn%20Object%20Reference) (NiagaraTemplate :type Niagara%20System%20Object%20Reference) (AttachToComponent :type Scene%20Component%20Object%20Reference) (AttachPointName :type Name) (Location :type Vector) (Rotation :type Rotator) (bAutoDestroy :type Boolean))
  (CallFunction|SpawnSystemAttachedMul LocalPawn NiagaraTemplate AttachToComponent AttachPointName Location Rotation bAutoDestroy))

(event Custom|SpawnEmitterAttached
  (params (ShouldReplicate :type Boolean) (LocalPawn :type Pawn%20Object%20Reference) (EmitterTemplate :type Particle%20System%20Object%20Reference) (AttachToComponent :type Scene%20Component%20Object%20Reference) (AttachPointName :type Name) (Location :type Vector) (Rotation :type Rotator) (Scale :type Vector) (bAutoDestroy :type Boolean))
  (Effects|SpawnEmitterAttached EmitterTemplate AttachToComponent AttachPointName Location Rotation Scale "KeepRelativeOffset" bAutoDestroy)
  (if ShouldReplicate
    (CallFunction|SpawnEmitterAttachedServer LocalPawn EmitterTemplate AttachToComponent AttachPointName Location Rotation Scale bAutoDestroy)))

(event Custom|SpawnEmitterAttachedServer
  (params (LocalPawn :type Pawn%20Object%20Reference) (EmitterTemplate :type Particle%20System%20Object%20Reference) (AttachToComponent :type Scene%20Component%20Object%20Reference) (AttachPointName :type Name) (Location :type Vector) (Rotation :type Rotator) (Scale :type Vector) (bAutoDestroy :type Boolean))
  (CallFunction|SpawnEmitterAttachedMul LocalPawn EmitterTemplate AttachToComponent AttachPointName Location Rotation Scale bAutoDestroy))

(event Custom|SpawnEmitterAttachedMul
  (params (LocalPawn :type Pawn%20Object%20Reference) (EmitterTemplate :type Particle%20System%20Object%20Reference) (AttachToComponent :type Scene%20Component%20Object%20Reference) (AttachPointName :type Name) (Location :type Vector) (Rotation :type Rotator) (Scale :type Vector) (bAutoDestroy :type Boolean))
  (if (not (Pawn|IsLocallyControlled LocalPawn))
    (Effects|SpawnEmitterAttached EmitterTemplate AttachToComponent AttachPointName Location Rotation Scale "KeepRelativeOffset" bAutoDestroy)))

(event Custom|SpawnSystemAtLocation
  (params (ShouldReplicate :type Boolean) (LocalPawn :type Pawn%20Object%20Reference) (SystemTemplate :type Niagara%20System%20Object%20Reference) (Location :type Vector) (Rotation :type Rotator) (Scale :type Vector) (bAutoDestroy :type Boolean))
  (Niagara|SpawnSystematLocation SystemTemplate Location Rotation Scale bAutoDestroy)
  (if ShouldReplicate
    (CallFunction|SpawnSystematLocationServer LocalPawn SystemTemplate Location Rotation Scale bAutoDestroy)))

(event Custom|SpawnSystemAtLocationServer
  (params (PlayerFormClient :type Pawn%20Object%20Reference) (SystemTemplate :type Niagara%20System%20Object%20Reference) (Location :type Vector) (Rotation :type Rotator) (Scale :type Vector) (bAutoDestroy :type Boolean))
  (CallFunction|SpawnSystematLocationMul PlayerFormClient SystemTemplate Location Rotation Scale bAutoDestroy))

(event Custom|SpawnSystemAtLocationMul
  (params (PlayerFromClient :type Pawn%20Object%20Reference) (SystemTemplate :type Niagara%20System%20Object%20Reference) (Location :type Vector) (Rotation :type Rotator) (Scale :type Vector) (bAutoDestroy :type Boolean))
  (if (not (Pawn|IsLocallyControlled PlayerFromClient))
    (Niagara|SpawnSystematLocation SystemTemplate Location Rotation Scale bAutoDestroy)))